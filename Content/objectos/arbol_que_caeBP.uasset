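; Choppable tree actor that shows a "cut me" prompt in the player's info widget when looked at.
; AnyDamage drains its health with an axe sound, using a Hit flag and short delay to throttle repeat hits.
; At low health it disables capsule collision, plays a falling sound and a Timeline that offsets the mesh vertically, then destroys itself.
; Interaction has no effect, and an older axe-collision damage path is left disconnected.
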(event `/Game/interact_interface.LookAt`
  (params (PlayerCharacter :type "/Game/ThirdPersonBP/Blueprints/ThirdPersonCharacter Object Reference"))
  (`/Game/widget/widget_pantalla_info.Update Message` (`/Game/ThirdPersonBP/Blueprints/ThirdPersonCharacter.widgetInfoItem` PlayerCharacter) (`|FormatText` "I'M  A TREE, CUT ME")))

(event `/Game/interact_interface.InteractWidth`
  (params (PlayerCharacter :type "/Game/ThirdPersonBP/Blueprints/ThirdPersonCharacter Object Reference"))
  (bind _output_get (set `self.player` PlayerCharacter))
  (`/Game/ThirdPersonBP/Blueprints/ThirdPersonCharacter.getCurremIten` _output_get
    (:`then`)
    (:`else`)))

(event `self.StaticMesh.OnComponentBeginOverlap`
  (params (OverlappedComponent :type "PrimitiveComponent Object Reference") (OtherActor :type "Actor Object Reference") (OtherComp :type "PrimitiveComponent Object Reference") (OtherBodyIndex :type Integer) (bFromSweep :type Boolean) (SweepResult :type "HitResult Structure (by ref)")))

(event `self.ReceiveAnyDamage`
  (params (Damage :type "Float (single-precision)") (DamageType :type "DamageType Object Reference") (InstigatedBy :type "Controller Object Reference") (DamageCauser :type "Actor Object Reference"))
  (if (not (`self.hit`))
    (set `self.hit` true)
    (bind _output_get (set `self.my_live` (- (`self.my_live`) Damage)))
    (`KismetSystemLibrary.PrintString` (`KismetStringLibrary.Conv_DoubleToString` _output_get))
    (`GameplayStatics.PlaySoundAtLocation` "/Game/sonidos/hacha.hacha" (`self.K2_GetActorLocation`) (struct) 1.0 1.0 0.0 null null null)
    (`KismetSystemLibrary.Delay` 0.2)
    (set `self.hit` false)
    (if (<= (`self.my_live`) 1.0)
      (if (not (`self.hit`))
        (set `self.hit` true)
        (`self.destruccion`)
        (`GameplayStatics.PlaySoundAtLocation` "/Game/sonidos/cae_Arbol.cae_Arbol" (`self.K2_GetActorLocation`) (struct) 1.0 1.0 0.0 null null null)
        (bind (_direction _newtrack_0) (`Timeline|caida`)
          (:`Update`
            (`SceneComponent.K2_AddLocalOffset` (`self.StaticMesh`) (`KismetMathLibrary.MakeVector` 0.0 0.0 _newtrack_0) false false))
          (:`Finished`
            (`KismetSystemLibrary.Delay` 2.2)
            (`self.K2_DestroyActor`)))))))

(event `self.Capsule.OnComponentBeginOverlap`
  (params (OverlappedComponent :type "PrimitiveComponent Object Reference") (OtherActor :type "Actor Object Reference") (OtherComp :type "PrimitiveComponent Object Reference") (OtherBodyIndex :type Integer) (bFromSweep :type Boolean) (SweepResult :type "HitResult Structure (by ref)")))

(event `self.Capsule.OnComponentHit`
  (params (HitComponent :type "PrimitiveComponent Object Reference") (OtherActor :type "Actor Object Reference") (OtherComp :type "PrimitiveComponent Object Reference") (NormalImpulse :type "Vector Structure") (Hit :type "HitResult Structure (by ref)")))

(fn `destruccion`
  (`PrimitiveComponent.SetCollisionEnabled` (`self.Capsule`) "NoCollision"))

(fn `UserConstructionScript`)