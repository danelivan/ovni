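; Axe weapon Blueprint that deals fixed damage to actors its Sphere component touches.
; The sphere's collision is disabled on BeginPlay and toggled through COLISIONONOFF, which also prints the new state on screen.
; Both hit and begin-overlap events on the sphere apply the same damage, with no filtering of the other actor or guard against repeated hits.
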(event `self.ReceiveBeginPlay`
  (`PrimitiveComponent.SetCollisionEnabled` (`self.Sphere`) "NoCollision"))

(event `self.Sphere.OnComponentHit`
  (params (HitComponent :type "PrimitiveComponent Object Reference") (OtherActor :type "Actor Object Reference") (OtherComp :type "PrimitiveComponent Object Reference") (NormalImpulse :type "Vector Structure") (Hit :type "HitResult Structure (by ref)"))
  (`GameplayStatics.ApplyDamage` OtherActor 50.0))

(event `self.Sphere.OnComponentBeginOverlap`
  (params (OverlappedComponent :type "PrimitiveComponent Object Reference") (OtherActor :type "Actor Object Reference") (OtherComp :type "PrimitiveComponent Object Reference") (OtherBodyIndex :type Integer) (bFromSweep :type Boolean) (SweepResult :type "HitResult Structure (by ref)"))
  (`GameplayStatics.ApplyDamage` OtherActor 50.0))

(fn `COLISIONONOFF`
  (params (on :type Boolean))
  (if on
    (`PrimitiveComponent.SetCollisionEnabled` (`self.Sphere`) "QueryAndPhysics")
    (`KismetSystemLibrary.PrintString` "colision activada")
    (else
      (`PrimitiveComponent.SetCollisionEnabled` (`self.Sphere`) "NoCollision")
      (`KismetSystemLibrary.PrintString` "colision desactivada"))))

(fn `UserConstructionScript`)