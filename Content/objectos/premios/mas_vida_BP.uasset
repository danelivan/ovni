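; Health pickup actor that restores part of the player's life on touch.
; The heart mesh spins by a fixed step every Tick, not scaled by delta time.
; Capsule overlap casts to ThirdPersonCharacter and, if MyLive is below the maximum, adds a clamped bonus and destroys the pickup.
; At full life the pickup stays in the world.
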(event `self.ReceiveTick`
  (params (DeltaSeconds :type "Float (single-precision)"))
  (`SceneComponent.K2_AddLocalRotation` (`self.HEART_heart_2`) (struct :`Yaw` 2.0) false false))

(event `self.Capsule.OnComponentBeginOverlap`
  (params (OverlappedComponent :type "PrimitiveComponent Object Reference") (OtherActor :type "Actor Object Reference") (OtherComp :type "PrimitiveComponent Object Reference") (OtherBodyIndex :type Integer) (bFromSweep :type Boolean) (SweepResult :type "HitResult Structure (by ref)"))
  (bind _asthird_person_character (cast `/Game/ThirdPersonBP/Blueprints/ThirdPersonCharacter` OtherActor))
  (if (< (`/Game/ThirdPersonBP/Blueprints/ThirdPersonCharacter.myLive` _asthird_person_character) 100.0)
    (set `/Game/ThirdPersonBP/Blueprints/ThirdPersonCharacter.myLive` (`KismetMathLibrary.FClamp` (+ (`/Game/ThirdPersonBP/Blueprints/ThirdPersonCharacter.myLive` _asthird_person_character) 30.0) 30.0 100.0) _asthird_person_character)
    (`self.K2_DestroyActor`)))

(fn `UserConstructionScript`)