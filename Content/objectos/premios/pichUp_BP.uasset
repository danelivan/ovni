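; Coin-style pickup that adds one to the ThirdPersonCharacter's Monedas count when touched.
; The Luz timeline, started on BeginPlay, drives the point light's intensity and offsets the actor from its start location, while Tick spins the root.
; Sphere overlap uses the Mepillo flag to award only once, spawns a fire hit effect, plays a ring sound and destroys the actor after a short delay.
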(event `self.ReceiveBeginPlay`
  (set `self.my_loc` (`self.K2_GetActorLocation`))
  (bind (_direction _newtrack_0 _up) (`Timeline|luz`)
    (:`Update`
      (`LightComponent.SetIntensity` (`self.PointLight`) _newtrack_0)
      (`self.K2_SetActorLocation` (+ (`self.my_loc`) _up))
      (`KismetSystemLibrary.Delay` 0.2))))

(event `self.ReceiveTick`
  (params (DeltaSeconds :type "Float (single-precision)"))
  (`SceneComponent.K2_AddLocalRotation` (`self.DefaultSceneRoot`) (struct :`Yaw` -2.0) false false))

(event `self.Sphere.OnComponentBeginOverlap`
  (params (OverlappedComponent :type "PrimitiveComponent Object Reference") (OtherActor :type "Actor Object Reference") (OtherComp :type "PrimitiveComponent Object Reference") (OtherBodyIndex :type Integer) (bFromSweep :type Boolean) (SweepResult :type "HitResult Structure (by ref)"))
  (bind _asthird_person_character (cast `/Game/ThirdPersonBP/Blueprints/ThirdPersonCharacter` OtherActor))
  (if (not (`self.mepillo?`))
    (set `self.mepillo?` true)
    (set `/Game/ThirdPersonBP/Blueprints/ThirdPersonCharacter.monedas` (+ (`/Game/ThirdPersonBP/Blueprints/ThirdPersonCharacter.monedas` _asthird_person_character) 1) _asthird_person_character)
    (`GameplayStatics.SpawnEmitterAtLocation` "/Game/AdvancedMagicFX12/particles/P_ky_hit_fire.P_ky_hit_fire" (`self.K2_GetActorLocation`))
    (`GameplayStatics.PlaySound2D` "/Game/Sounds/Ring_Cue.Ring_Cue" 1.0 1.0 0.0 null null)
    (`KismetSystemLibrary.Delay` 0.2)
    (`self.K2_DestroyActor`)))

(fn `UserConstructionScript`)