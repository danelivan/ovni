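; Spring actor that launches the ThirdPersonCharacter straight up when it hits the Box component.
; On hit it sets the character's flying and falling flags, calls its FINISHVOLAR and DetectarSuelo functions, applies an upward force plus a velocity-change impulse, and plays a spring sound.
; BeginPlay computes a signed Angle from the actor's orientation, but the launch ignores it and always pushes along world Z.
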(event `self.ReceiveBeginPlay`
  (bind _returnvalue (`KismetMathLibrary.SignOfFloat` (.z (`KismetMathLibrary.Cross_VectorVector` (`self.GetActorRightVector`) (`self.GetActorUpVector`)))))
  (set `self.Angle` (* (`KismetMathLibrary.Acos` (`KismetMathLibrary.Dot_VectorVector` (`KismetMathLibrary.Cross_VectorVector` (`self.GetActorRightVector`) (`self.GetActorForwardVector`)) (0.0 0.0 1.0))) (select `bool` (== _returnvalue 0.0) :`false` _returnvalue :`true` 1.0))))

(event `self.Box.OnComponentHit`
  (params (HitComponent :type "PrimitiveComponent Object Reference") (OtherActor :type "Actor Object Reference") (OtherComp :type "PrimitiveComponent Object Reference") (NormalImpulse :type "Vector Structure") (Hit :type "HitResult Structure (by ref)"))
  (bind _asthird_person_character (cast `/Game/ThirdPersonBP/Blueprints/ThirdPersonCharacter` OtherActor))
  (set `/Game/ThirdPersonBP/Blueprints/ThirdPersonCharacter.volando?` true _asthird_person_character)
  (set `/Game/ThirdPersonBP/Blueprints/ThirdPersonCharacter.cayendo` true _asthird_person_character)
  (`/Game/ThirdPersonBP/Blueprints/ThirdPersonCharacter.FINISHVOLAR` _asthird_person_character)
  (`/Game/ThirdPersonBP/Blueprints/ThirdPersonCharacter.detectar Suelo` _asthird_person_character)
  (bind _charactermovement (`Character.CharacterMovement` _asthird_person_character))
  (`CharacterMovementComponent.AddForce` _charactermovement (0.0 0.0 100.0))
  (`CharacterMovementComponent.AddImpulse` _charactermovement (0.0 0.0 1100.0) true)
  (`GameplayStatics.PlaySound2D` "/Game/sonidos/Spring.Spring" 1.0 1.0 0.0 null null))

(fn `UserConstructionScript`)