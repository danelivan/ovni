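; A destructible actor, named as a vanishing platform, that shatters when the ThirdPersonCharacter hits it.
; The first hit applies damage with an impulse, spawns smoke, plays a boom, then destroys the emitter and actor after a delay.
; Later character hits still apply damage, but a Broken flag guards the one-time effects.
; Tick updates a DeathTimer once broken, though its timer-based destroy branch is unconnected.
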(event `self.ReceiveBeginPlay`
  (bind _asthird_person_character (cast `/Game/ThirdPersonBP/Blueprints/ThirdPersonCharacter` (`GameplayStatics.GetPlayerPawn` 0)))
  (set `self.Player` _asthird_person_character))

(event `self.ReceiveTick`
  (params (DeltaSeconds :type "Float (single-precision)"))
  (set `self.DeltaTime` DeltaSeconds)
  (`|ExecutionSequence`
    (:`then_0`
      ;[1 1 1] Destroy pieces
      (if (`self.Broken`)
        (`|ExecutionSequence`
          (:`then_0`
            (set `self.DeathTimer` (* (+ (`self.DeathTimer`) 1.0) (/ (`self.DeltaTime`) 0.016)))))))))

(event `self.Destructible.OnComponentHit`
  (params (HitComponent :type "PrimitiveComponent Object Reference") (OtherActor :type "Actor Object Reference") (OtherComp :type "PrimitiveComponent Object Reference") (NormalImpulse :type "Vector Structure") (Hit :type "HitResult Structure (by ref)"))
  (cast `/Game/ThirdPersonBP/Blueprints/ThirdPersonCharacter` OtherActor)
  (`DestructibleComponent.ApplyDamage` (`self.Destructible`) 1.0 Hit_Location Hit_ImpactPoint 10000.0)
  (if (not (`self.Broken`))
    (set `self.Broken` true)
    (bind _returnvalue (`GameplayStatics.SpawnEmitterAtLocation` "/Game/MobileStarterContent/Particles/P_Smoke.P_Smoke" (`self.K2_GetActorLocation`)))
    (`GameplayStatics.PlaySoundAtLocation` "/Game/sonidos/boom.boom" (0.0 0.0 0.0) (struct) 1.0 1.0 0.0 null null null)
    (`KismetSystemLibrary.Delay` 5.0)
    (`ActorComponent.K2_DestroyComponent` _returnvalue)
    (`self.K2_DestroyActor`)))

(fn `UserConstructionScript`)