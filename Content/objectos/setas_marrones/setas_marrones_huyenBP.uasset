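; Brown mushroom creature that flees when its AI perception senses the ThirdPersonCharacter.
; The first successful sensing sets the Corriendo flag, which is never reset here, and calls HUIMOS.
; HUIMOS applies only the pitch of the look-at rotation toward the player, then calls AIMoveTo.
; The destination is a fixed world point with X set to Distanciapatras, independent of mushroom or player position.
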(event `HUIMOS`
  (bind _asthird_person_character (cast `/Game/ThirdPersonBP/Blueprints/ThirdPersonCharacter` (`GameplayStatics.GetPlayerCharacter` 0)))
  (bind (_returnvalue_roll _returnvalue_pitch) (`KismetMathLibrary.BreakRotator` (`KismetMathLibrary.FindLookAtRotation` (`self.K2_GetActorLocation`) (`self.K2_GetActorLocation` _asthird_person_character))))
  (`self.K2_SetActorRotation` (`KismetMathLibrary.MakeRotator` 0.0 _returnvalue_pitch))
  (`|AIMoveTo` self (`KismetMathLibrary.MakeVector` (`self.distanciapatras`)) null))

(event `self.AIPerception.OnTargetPerceptionUpdated`
  (params (Actor :type "Actor Object Reference") (Stimulus :type "AIStimulus Structure"))
  (cast `/Game/ThirdPersonBP/Blueprints/ThirdPersonCharacter` Actor)
  (if (`.bSuccessfullySensed` (break `AIStimulus` Stimulus))
    (`KismetSystemLibrary.PrintString` "POR PATAS")
    (if (not (`self.corriendo?`))
      (set `self.corriendo?` true)
      (`self.HUIMOS`))))

(fn `UserConstructionScript`)