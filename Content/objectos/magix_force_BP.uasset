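; Magic power pickup actor, presented as a "magic potato", that raises the player's magic power.
; When a ThirdPersonCharacter overlaps its Box, it adds its Power value to that character's PowerMagic, spawns a water-hit particle effect and destroys itself after a short delay.
; Its Lookat event writes the potato message to the player's item info widget.
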(event `/Game/interact_interface.LookAt`
  (params (PlayerCharacter :type "/Game/ThirdPersonBP/Blueprints/ThirdPersonCharacter Object Reference"))
  (`/Game/widget/widget_pantalla_info.Update Message` (`/Game/ThirdPersonBP/Blueprints/ThirdPersonCharacter.widgetInfoItem` PlayerCharacter) (`|FormatText` "I am a MAGIC POTATO, GET ME!")))

(event `self.Box.OnComponentBeginOverlap`
  (params (OverlappedComponent :type "PrimitiveComponent Object Reference") (OtherActor :type "Actor Object Reference") (OtherComp :type "PrimitiveComponent Object Reference") (OtherBodyIndex :type Integer) (bFromSweep :type Boolean) (SweepResult :type "HitResult Structure (by ref)"))
  (bind _asthird_person_character (cast `/Game/ThirdPersonBP/Blueprints/ThirdPersonCharacter` OtherActor))
  (set `/Game/ThirdPersonBP/Blueprints/ThirdPersonCharacter.powerMagic` (+ (`/Game/ThirdPersonBP/Blueprints/ThirdPersonCharacter.powerMagic` _asthird_person_character) (`self.power`)) _asthird_person_character)
  (`GameplayStatics.SpawnEmitterAtLocation` "/Game/AdvancedMagicFX12/particles/P_ky_hit_water.P_ky_hit_water" (`self.K2_GetActorLocation`))
  (`KismetSystemLibrary.Delay` 0.2)
  (`self.K2_DestroyActor`))

(fn `UserConstructionScript`)