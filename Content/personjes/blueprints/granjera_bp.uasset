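; Farmer NPC that works as either a sower or a harvester, chosen by ClaseActor on BeginPlay.
; Sowers loop between random navmesh points around their start, pausing with Sembrando set.
; Harvesters show a basket and cycle via AIMoveTo between the nearest fruit tree, home and nearest tomato plant, setting gathering flags.
; Failed harvest moves or any actor overlap trigger a move-home fallback into harvesting; Tick clears the greeting flag.
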(event `self.ReceiveBeginPlay`
  ;[1 1 1] INICIO SETUP PERSONAJE
  (`|ExecutionSequence`
    (:`then_0`
      (`SceneComponent.SetVisibility` (`self.cesta`) false false)
      (set `self.my_loc` (`self.K2_GetActorLocation`))
      (set `CharacterMovementComponent.MaxWalkSpeed` 200.0 (`self.CharacterMovement`))
      (switch `int` (`self.claseActor`)
        (:`Default`
          (`self.ando_Sembrado`))
        (:`0`
          (`self.ando_Sembrado`))
        (:`1`
          (`SceneComponent.SetVisibility` (`self.cesta`) true false)
          (`self.ando_recogiendo`))))
    (:`then_1`
      (bind _asmy_game_instance (cast `/Game/variables_y_controladores/my_game_instance` (`GameplayStatics.GetGameInstance`)))
      (set `self.instanceGame` _asmy_game_instance))))

(event `ando_recogiendo`
  ;[1 1 1] SOY RECOLECTOR
  (bind _outactors (`GameplayStatics.GetAllActorsOfClass` "/Game/objectos/arbol_frutal/arbol_frutal.arbol_frutal_C"))
  (bind _actor_close (`self.Findarbolcerca` _outactors))
  (set `self.myarbol` _actor_close)
  (bind _outactors_2 (`GameplayStatics.GetAllActorsOfClass` "/Game/objectos/arbol_frutal/tomateras.tomateras_C"))
  (bind _actor_close_2 (`self.Findarbolcerca` _outactors_2))
  (set `self.my_tomatera` _actor_close_2)
  (`self.recolecto`))

(event `recolecto`
  ;[1 1 1] RECOLECTABNDO LOOP
  (`|AIMoveTo` self (0.0 0.0 0.0) (`self.myarbol`) :!label _label
    (:`OnSuccess`
      (set `self.recogiendo arbol?` true)
      (`KismetSystemLibrary.Delay` (`KismetMathLibrary.RandomFloatInRange` 8.0 15.0))
      (set `self.recogiendo arbol?` false)
      (`|AIMoveTo` self (`self.my_loc`) null
        (:`OnSuccess`
          (`KismetSystemLibrary.Delay` (`KismetMathLibrary.RandomFloatInRange` 8.0 15.0))
          (`|AIMoveTo` self (0.0 0.0 0.0) (`self.my_tomatera`)
            (:`OnSuccess`
              (set `self.recogiendo arbusto?` true)
              (`KismetSystemLibrary.Delay` (`KismetMathLibrary.RandomFloatInRange` 8.0 15.0))
              (set `self.recogiendo arbusto?` false)
              (`|AIMoveTo` self (`self.my_loc`) null
                (:`OnSuccess`
                  (`KismetSystemLibrary.Delay` (`KismetMathLibrary.RandomFloatInRange` 8.0 15.0))
                  (goto _label))))
            (:`OnFail`
              (`self.NO LLEGO A RECOLECTAR`))))))
    (:`OnFail`
      (`self.NO LLEGO A RECOLECTAR`))))

(event `NO LLEGO A RECOLECTAR`
  ;[1 1 1] NO LLEGO A RECOLECTAR
  (`|AIMoveTo` null (`self.my_loc`) null
    (:`OnSuccess`
      _)
    (:`OnFail`
      _))
  (`self.recolecto`))

(event `self.ReceiveActorBeginOverlap`
  (params (OtherActor :type "Actor Object Reference"))
  ;[1 1 1] COLLISION
  (`self.NO LLEGO A RECOLECTAR`))

(event `ando_Sembrado`
  ;[1 1 1] SOY SEMBRADOR
  (bind _randomlocation (`NavigationSystemV1.K2_GetRandomLocationInNavigableRadius` (`self.my_loc`) 1500.0 null null :!label _label_2))
  (`|AIMoveTo` self _randomlocation null
    (:`OnSuccess`
      (set `self.sembrando?` true)
      (`KismetSystemLibrary.Delay` (`KismetMathLibrary.RandomFloatInRange` 8.0 20.0))
      (set `self.my_time` (+ (`self.my_time`) 1))
      (set `self.sembrando?` false)
      (if (>= (`self.my_time`) 3)
        (set `self.my_time` 0)
        (`KismetSystemLibrary.Delay` 5.0)
        (goto _label_2)
        (else
          (goto _label_2))))))

(event `self.ReceiveTick`
  (params (DeltaSeconds :type "Float (single-precision)"))
  (`|ExecutionSequence`
    (:`then_0`
      (if (`self.salutatis`)
        (set `self.time_salutatis` (+ (`self.time_salutatis`) 1))
        (if (> (`self.time_salutatis`) 10)
          (set `self.time_salutatis` 0)
          (set `self.salutatis` false))))))

(fn `Findarbolcerca`
  (params (actor :type "Array of Actor Object Reference"))
  (returns (`actor close` :type "Actor Object Reference"))
  (for _array_element actor
    (`KismetArrayLibrary.Array_Add` (`self.Local Distance`) (`KismetMathLibrary.Vector_Distance` (`self.K2_GetActorLocation` _array_element) (`self.K2_GetActorLocation`))))
  (return (`|GetArrayItem` actor (`KismetMathLibrary.MinOfFloatArray` (`self.Local Distance`)))))

(fn `UserConstructionScript`)