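; Ambient NPC pawn that loops through a routine between its spawn point, a market stall, sacks and a Negreta_bp actor.
; On BeginPlay it stores its position and caches the nearest actor of each target class by distance.
; Chained AIMoveTo calls and delays drive the loop, setting activity flags at stall and sacks; failed moves send it home before restarting.
; A separate random-radius Patrullar event is never called in this graph.
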(event `self.ReceiveBeginPlay`
  (set `self.pos_loc` (`self.K2_GetActorLocation`))
  (`self.setup_localizaciones`))

(event `setup_localizaciones`
  (bind _outactors (`GameplayStatics.GetAllActorsOfClass` "/Game/personjes/blueprints/tenderete_bp.tenderete_bp_C"))
  (bind _actor (`self.buscarlomascerca` _outactors))
  (set `self.tenderete` _actor)
  (bind _outactors_2 (`GameplayStatics.GetAllActorsOfClass` "/Game/personjes/blueprints/sacos_bp.sacos_bp_C"))
  (bind _actor_2 (`self.buscarlomascerca` _outactors_2))
  (set `self.sacos` _actor_2)
  (bind _outactors_3 (`GameplayStatics.GetAllActorsOfClass` "/Game/personjes/blueprints/negreta_bp.negreta_bp_C"))
  (bind _actor_3 (`self.buscarlomascerca` _outactors_3))
  (set `self.negreta` _actor_3)
  (`self.bucle_andar`))

(event `Patrullar`
  (bind _randomlocation (`NavigationSystemV1.K2_GetRandomLocationInNavigableRadius` (`self.pos_loc`) (`self.radio_andar`) null null :!label _label))
  (`|AIMoveTo` self _randomlocation null
    (:`OnSuccess`
      (`KismetSystemLibrary.Delay` 5.0)
      (goto _label))))

(event `bucle_andar`
  (`|AIMoveTo` self (0.0 0.0 0.0) (`self.tenderete`) 40.0 :!label _label_2
    (:`OnSuccess`
      (set `self.comprando?` true)
      (`KismetSystemLibrary.Delay` (`KismetMathLibrary.RandomFloatInRange` 5.0 12.0))
      (set `self.comprando?` false)
      (`|AIMoveTo` self (`self.pos_loc`) null 30.0
        (:`OnSuccess`
          (`KismetSystemLibrary.Delay` (`KismetMathLibrary.RandomFloatInRange` 2.0 4.0))
          (`|AIMoveTo` self (0.0 0.0 0.0) (`self.sacos`) 40.0
            (:`OnSuccess`
              (set `self.bonitobicho?` true)
              (`KismetSystemLibrary.Delay` (`KismetMathLibrary.RandomFloatInRange` 3.0 5.0))
              (set `self.bonitobicho?` false)
              (`|AIMoveTo` self (`self.pos_loc`) null 10.0
                (:`OnSuccess`
                  (`KismetSystemLibrary.Delay` 2.0)
                  (`|AIMoveTo` self (0.0 0.0 0.0) (`self.negreta`) 60.0
                    (:`OnSuccess`
                      (`KismetSystemLibrary.Delay` 1.5)
                      (`KismetSystemLibrary.Delay` 2.0)
                      (goto _label_2))
                    (:`OnFail`
                      (`self.vuelvoalsitio`))))
                (:`OnFail`
                  (`self.vuelvoalsitio`))))
            (:`OnFail`
              (`self.vuelvoalsitio`))))
        (:`OnFail`
          (`self.vuelvoalsitio`))))
    (:`OnFail`
      (`self.vuelvoalsitio`))))

(event `vuelvoalsitio`
  (`|AIMoveTo` self (`self.pos_loc`) null
    (:`OnSuccess`
      (set `self.comprando?` false)
      (set `self.aplaudo?` false)
      (set `self.bonitobicho?` false))
    (:`OnFail`
      _))
  (`self.bucle_andar`))

(fn `buscarlomascerca`
  (params (actores :type "Array of Actor Object Reference"))
  (returns (actor :type "Actor Object Reference"))
  (for _array_element actores
    (`KismetArrayLibrary.Array_Add` (`self.Local Distance`) (`KismetMathLibrary.Vector_Distance` (`self.K2_GetActorLocation` _array_element) (`self.K2_GetActorLocation`))))
  (return (`|GetArrayItem` actores (`KismetMathLibrary.MinOfFloatArray` (`self.Local Distance`)))))

(fn `UserConstructionScript`)