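; Pumpkin prize pickup that pays a random number of coins to the ThirdPersonCharacter that hits its sphere.
; On hit it disables sphere collision, hides the coin particle, then loops on a short delay, adding to Monedas and spawning a COIN_BP each step.
; It destroys itself when the prize runs out, or when a per-tick MyLive countdown expires, even mid-payout.
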(event `self.ReceiveBeginPlay`
  (set `self.my_premio` (`KismetMathLibrary.RandomIntegerInRange` 10 50))
  (`Timeline|upSpmbrero`))

(event `self.Sphere.OnComponentHit`
  (params (HitComponent :type "PrimitiveComponent Object Reference") (OtherActor :type "Actor Object Reference") (OtherComp :type "PrimitiveComponent Object Reference") (NormalImpulse :type "Vector Structure") (Hit :type "HitResult Structure (by ref)"))
  (bind _asthird_person_character (cast `/Game/ThirdPersonBP/Blueprints/ThirdPersonCharacter` OtherActor))
  (`PrimitiveComponent.SetCollisionEnabled` (`self.Sphere`) "NoCollision")
  (`SceneComponent.SetVisibility` (`self.coin_particle`) false true)
  (set `self.my_premio` (- (`self.my_premio`) 1) :!label _label)
  (set `/Game/ThirdPersonBP/Blueprints/ThirdPersonCharacter.monedas` (+ (`/Game/ThirdPersonBP/Blueprints/ThirdPersonCharacter.monedas` _asthird_person_character) 1) _asthird_person_character)
  (`|SpawnActorFromClass` "/Game/ivan/COIN_BP.COIN_BP_C" (`self.GetTransform`) "Undefined" "OverrideRootScale" null null)
  (`KismetSystemLibrary.Delay` 0.2)
  (if (> (`self.my_premio`) 0)
    (goto _label)
    (else
      (`KismetSystemLibrary.PrintString` "DESTRUYO ACTOR")
      (`self.K2_DestroyActor`))))

(event `self.ReceiveTick`
  (params (DeltaSeconds :type "Float (single-precision)"))
  (set `self.my_live` (- (`self.my_live`) 1))
  (if (<= (`self.my_live`) 0)
    (`self.K2_DestroyActor`)))

(fn `UserConstructionScript`)