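; Calabaza is an enemy AI character with a constantly spinning Tapadera component, which chases the player's ThirdPersonCharacter on sight.
; PawnSensing detection turns on its point light, raises the mesh, switches movement to flying and runs AIMoveTo toward the player.
; When the chase succeeds (after a short delay) or fails, it darkens, resumes walking and returns to its BeginPlay location.
; Each Sphere hit costs a life, and at zero it explodes and is destroyed.
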(event `self.ReceiveBeginPlay`
  (`|ExecutionSequence`
    (:`then_0`
      (`LightComponent.SetIntensity` (`self.PointLight`) 0.0))
    (:`then_1`
      (set `self.my_loc` (`self.K2_GetActorLocation`)))))

(event `self.ReceiveTick`
  (params (DeltaSeconds :type "Float (single-precision)"))
  (`SceneComponent.K2_AddLocalRotation` (`self.tapadera`) (struct :`Yaw` -2.0) false false))

(event `self.PawnSensing.OnSeePawn`
  (params (Pawn :type "Pawn Object Reference"))
  ;[1 1 1] DETECTION
  (bind _asthird_person_character (cast `/Game/ThirdPersonBP/Blueprints/ThirdPersonCharacter` Pawn))
  (`LightComponent.SetIntensity` (`self.PointLight`) 50000.0)
  (`SceneComponent.K2_AddLocalOffset` (`self.Mesh`) (0.0 0.0 10.0) false false)
  (`CharacterMovementComponent.SetMovementMode` (`self.CharacterMovement`) "MOVE_Flying" 0)
  (`|AIMoveTo` self (0.0 0.0 0.0) _asthird_person_character 80.0
    (:`OnSuccess`
      (`KismetSystemLibrary.Delay` 1.0)
      (`SceneComponent.K2_AddLocalOffset` (`self.Mesh`) (0.0 0.0 0.0) false false)
      (`CharacterMovementComponent.SetMovementMode` (`self.CharacterMovement`) "MOVE_Walking" 0)
      (`LightComponent.SetIntensity` (`self.PointLight`) 0.0)
      (`|AIMoveTo` null (`self.my_loc`) null))
    (:`OnFail`
      (`SceneComponent.K2_AddLocalOffset` (`self.Mesh`) (0.0 0.0 0.0) false false)
      (`CharacterMovementComponent.SetMovementMode` (`self.CharacterMovement`) "MOVE_Walking" 0)
      (`LightComponent.SetIntensity` (`self.PointLight`) 0.0)
      (`|AIMoveTo` null (`self.my_loc`) null))))

(event `self.Sphere.OnComponentHit`
  (params (HitComponent :type "PrimitiveComponent Object Reference") (OtherActor :type "Actor Object Reference") (OtherComp :type "PrimitiveComponent Object Reference") (NormalImpulse :type "Vector Structure") (Hit :type "HitResult Structure (by ref)"))
  (set `self.my_live` (- (`self.my_live`) 1))
  (if (<= (`self.my_live`) 0)
    (`GameplayStatics.SpawnEmitterAtLocation` "/Game/MobileStarterContent/Particles/P_Explosion.P_Explosion" (`self.K2_GetActorLocation`))
    (`KismetSystemLibrary.Delay` 0.2)
    (`self.K2_DestroyActor`)))

(fn `UserConstructionScript`)