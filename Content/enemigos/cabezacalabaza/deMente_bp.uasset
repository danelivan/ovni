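; deMente_bp is a switchable damage hazard among the pumpkin-head enemy assets, built from a collision sphere and a particle effect.
; ROCKoNoFF turns the sphere's collision and the particle visibility on or off together, and records the state in the Ataco flag.
; While collision is on, sphere hits apply fixed damage to a ThirdPersonCharacter.
; BeginPlay hides only the particles, leaving collision at its default.
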(event `self.Sphere.OnComponentHit`
  (params (HitComponent :type "PrimitiveComponent Object Reference") (OtherActor :type "Actor Object Reference") (OtherComp :type "PrimitiveComponent Object Reference") (NormalImpulse :type "Vector Structure") (Hit :type "HitResult Structure (by ref)"))
  (bind _asthird_person_character (cast `/Game/ThirdPersonBP/Blueprints/ThirdPersonCharacter` OtherActor))
  (`GameplayStatics.ApplyDamage` _asthird_person_character 45.0))

(event `self.ReceiveBeginPlay`
  (`SceneComponent.SetVisibility` (`self.ParticleSystem`) false false))

(fn `ROCKoNoFF`
  (params (status :type Boolean))
  (if status
    (`PrimitiveComponent.SetCollisionEnabled` (`self.Sphere`) "QueryAndPhysics")
    (`SceneComponent.SetVisibility` (`self.ParticleSystem`) true false)
    (set `self.ataco` true)
    (else
      (`PrimitiveComponent.SetCollisionEnabled` (`self.Sphere`) "NoCollision")
      (`SceneComponent.SetVisibility` (`self.ParticleSystem`) false false)
      (set `self.ataco` false))))

(fn `UserConstructionScript`)