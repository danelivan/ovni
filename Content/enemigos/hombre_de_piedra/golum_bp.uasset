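; Stone golem enemy Blueprint that wanders the navmesh endlessly from BeginPlay.
; Its andnado event picks a random navigable point within a radius of itself, randomly sets a slower or faster walk speed through ChangueMovement, then calls AIMoveTo.
; On success it sets Finde, waits briefly and repeats; a failed move does not restart the loop, and the Atacando check is unconnected.
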(event `self.ReceiveBeginPlay`
  (`self.andnado`))

(event `andnado`
  ;[1 1 1] ANDAR
  (bind _randomlocation (`NavigationSystemV1.K2_GetRandomLocationInNavigableRadius` (`self.K2_GetActorLocation`) 1500.0 null null :!label _label))
  (`self.changue_Movement` (`KismetMathLibrary.RandomIntegerInRange` 1 2))
  (`|AIMoveTo` self _randomlocation null
    (:`OnSuccess`
      (set `self.finde` true)
      (`KismetSystemLibrary.Delay` 1.0)
      (goto _label))))

(fn `changue_Movement`
  (params (pos :type Integer))
  (if (== pos 1)
    (bind _output_get (set `self.speed` 200.0))
    (set `CharacterMovementComponent.MaxWalkSpeed` _output_get (`self.CharacterMovement`))
    (else
      (bind _output_get_2 (set `self.speed` 400.0))
      (set `CharacterMovementComponent.MaxWalkSpeed` _output_get_2 (`self.CharacterMovement`)))))

(fn `UserConstructionScript`)