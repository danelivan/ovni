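; Pumpkin enemy character that detects, shoots and chases the player, taking damage until it explodes and is destroyed.
; PawnSensing lights it up, switches it to flying, fires a projectile if the player is close, then runs AIMoveTo, later returning to its spawn location on foot.
; Tick spins the lid and updates a health-bar widget yawed toward the player.
; If HaveLive is set, a one-second looping timer destroys it after 600 counts.
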(event `self.ReceiveBeginPlay`
  (`|ExecutionSequence`
    (:`then_0`
      (`LightComponent.SetIntensity` (`self.PointLight`) 0.0))
    (:`then_1`
      (set `self.my_loc` (`self.K2_GetActorLocation`)))
    (:`then_2`
      (if (`self.haveLive?`)
        (`KismetSystemLibrary.K2_SetTimer` null "KillMe" 1.0 true)))))

(event `DISPARO`
  (bind _returnvalue (`self.GetDistanceTo` (`GameplayStatics.GetPlayerCharacter` 0) self))
  (bind (_returnvalue_location _returnvalue_rotation) (`KismetMathLibrary.BreakTransform` (`KismetMathLibrary.MakeTransform` (`SceneComponent.K2_GetComponentLocation` (`self.Arrow1`)) (`self.GetControlRotation`))))
  ;[1 1 1] disparo
  (set `self.mydistancia` _returnvalue)
  (if (<= _returnvalue 550.0)
    (`|SpawnActorFromClass` "/Game/enemigos/calabaza/projectil_calabazas.projectil_calabazas_C" (`KismetMathLibrary.MakeTransform` _returnvalue_location _returnvalue_rotation (0.5 0.5 0.5)) "Undefined" "OverrideRootScale" null null)))

(event `self.PawnSensing.OnSeePawn`
  (params (Pawn :type "Pawn Object Reference"))
  ;[1 1 1] DETECTION
  (bind _asthird_person_character (cast `/Game/ThirdPersonBP/Blueprints/ThirdPersonCharacter` Pawn))
  (`LightComponent.SetIntensity` (`self.PointLight`) 50000.0)
  (`SceneComponent.K2_AddLocalOffset` (`self.Mesh`) (0.0 0.0 10.0) false false)
  (`CharacterMovementComponent.SetMovementMode` (`self.CharacterMovement`) "MOVE_Flying" 0)
  (`self.DISPARO`)
  (`|AIMoveTo` self (0.0 0.0 0.0) _asthird_person_character 90.0 true
    (:`OnSuccess`
      (`SceneComponent.K2_AddLocalOffset` (`self.Mesh`) (0.0 0.0 0.0) false false)
      (`CharacterMovementComponent.SetMovementMode` (`self.CharacterMovement`) "MOVE_Walking" 0)
      (`LightComponent.SetIntensity` (`self.PointLight`) 0.0)
      (`|AIMoveTo` null (`self.my_loc`) null
        (:`then`
          (`KismetSystemLibrary.RetriggerableDelay` 1.0)
          (`SceneComponent.K2_AddLocalOffset` (`self.Mesh`) (0.0 0.0 0.0) false false)
          (`CharacterMovementComponent.SetMovementMode` (`self.CharacterMovement`) "MOVE_Walking" 0)
          (`LightComponent.SetIntensity` (`self.PointLight`) 0.0)
          (`|AIMoveTo` null (`self.my_loc`) null))))
    (:`OnFail`
      (`SceneComponent.K2_AddLocalOffset` (`self.Mesh`) (0.0 0.0 0.0) false false)
      (`CharacterMovementComponent.SetMovementMode` (`self.CharacterMovement`) "MOVE_Walking" 0)
      (`LightComponent.SetIntensity` (`self.PointLight`) 0.0)
      (`|AIMoveTo` null (`self.my_loc`) null))))

(event `self.ReceiveTick`
  (params (DeltaSeconds :type "Float (single-precision)"))
  ;[1 1 1] EVENTO TICK
  (`|ExecutionSequence`
    (:`then_0`
      (`SceneComponent.K2_AddLocalRotation` (`self.tapadera`) (struct :`Yaw` -2.0) false false))
    (:`then_1`
      (bind _aswdget_live (cast `/Game/widget/wdget_live` (`WidgetComponent.GetUserWidgetObject` (`self.Widget`))))
      (`ProgressBar.SetPercent` (`/Game/widget/wdget_live.proLive` _aswdget_live) (/ (`self.my_live`) 100.0))
      (`SceneComponent.K2_SetWorldRotation` (`self.Widget`) (`KismetMathLibrary.MakeRotator` 0.0 0.0 (.yaw (`KismetMathLibrary.FindLookAtRotation` (`SceneComponent.K2_GetComponentLocation` (`self.Widget`)) (`self.K2_GetActorLocation` (`GameplayStatics.GetPlayerCharacter` 0))))) false false))))

(event `self.ReceiveAnyDamage`
  (params (Damage :type "Float (single-precision)") (DamageType :type "DamageType Object Reference") (InstigatedBy :type "Controller Object Reference") (DamageCauser :type "Actor Object Reference"))
  ;[1 1 1] EVENTO DAMAGE
  (`KismetSystemLibrary.PrintString` "mas dado" true true (struct :`R` 1.0 :`G` 0.969005 :`A` 1.0))
  (set `self.my_live` (- (`self.my_live`) Damage))
  (`GameplayStatics.SpawnEmitterAtLocation` "/Game/MobileStarterContent/Particles/P_Explosion.P_Explosion" (`self.K2_GetActorLocation`))
  (if (<= (`self.my_live`) 0.0)
    (`GameplayStatics.SpawnEmitterAtLocation` "/Game/FXVarietyPack/Particles/P_ky_shotShockwave.P_ky_shotShockwave" (`self.K2_GetActorLocation`))
    (`GameplayStatics.SpawnEmitterAtLocation` "/Game/FXVarietyPack/Particles/P_ky_ThunderBallHit.P_ky_ThunderBallHit" (`self.K2_GetActorLocation`))
    (`KismetSystemLibrary.Delay` 0.2)
    (`self.K2_DestroyActor`)))

(fn `killMe`
  (set `self.sumaSegundo` (+ (`self.sumaSegundo`) 1))
  (if (>= (`self.sumaSegundo`) 600)
    (`self.K2_DestroyActor`)))

(fn `UserConstructionScript`)