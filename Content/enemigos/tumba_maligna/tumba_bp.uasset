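; Evil tomb Blueprint (tumba maligna) that spawns a random actor when the player's ThirdPersonCharacter enters its Box.
; The overlap plays an explosion effect and Risas_cue sound, shuffles the MyActor class array, then waits briefly.
; It then spawns one of three entries at the Arrow's transform and stores it in Elactorcreado.
; MyBixo blocks further triggers, but is only set after the spawn, so re-entry during the delay repeats the effects.
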(event `self.ReceiveActorBeginOverlap`
  (params (OtherActor :type "Actor Object Reference")))

(event `self.Box.OnComponentBeginOverlap`
  (params (OverlappedComponent :type "PrimitiveComponent Object Reference") (OtherActor :type "Actor Object Reference") (OtherComp :type "PrimitiveComponent Object Reference") (OtherBodyIndex :type Integer) (bFromSweep :type Boolean) (SweepResult :type "HitResult Structure (by ref)"))
  (bind _my_actor (`self.my_actor`))
  (cast `/Game/ThirdPersonBP/Blueprints/ThirdPersonCharacter` OtherActor)
  (if (not (`self.my_bixo`))
    (`GameplayStatics.SpawnEmitterAtLocation` "/Game/MobileStarterContent/Particles/P_Explosion.P_Explosion" (`self.K2_GetActorLocation`) (struct) (5.0 5.0 5.0))
    (`KismetArrayLibrary.Array_Shuffle` _my_actor)
    (`GameplayStatics.PlaySoundAtLocation` "/Game/sonidos/risas/risas_cue.risas_cue" (`self.K2_GetActorLocation`) (struct) 1.0 1.0 0.0 null null null)
    (`KismetSystemLibrary.Delay` 1.0)
    (bind _returnvalue (`|SpawnActorFromClass` (`|GetArrayItem` _my_actor (`KismetMathLibrary.RandomIntegerInRange` 0 2)) (`SceneComponent.K2_GetComponentToWorld` (`self.Arrow`)) "Undefined" "OverrideRootScale" null null))
    (set `self.elactorcreado` _returnvalue)
    (set `self.my_bixo` true)))

(fn `UserConstructionScript`)