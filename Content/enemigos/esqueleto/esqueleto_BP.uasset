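; Skeleton enemy character that takes damage and attacks by spawning a projectile.
; BeginPlay sets MyUz intensity to zero, and AnyDamage raises Hit, subtracts from MyLife and raises Die when life runs out.
; Velocidad sets max walk speed, while Atacando either spawns Proyectil_esqueleto_prqueBP at Arrow1 or clears the Ataco flag, depending on Status.
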(event `self.ReceiveBeginPlay`
  (`LightComponent.SetIntensity` (`self.my_uz`) 0.0))

(event `self.ReceiveAnyDamage`
  (params (Damage :type "Float (single-precision)") (DamageType :type "DamageType Object Reference") (InstigatedBy :type "Controller Object Reference") (DamageCauser :type "Actor Object Reference"))
  (set `self.hit?` true)
  (set `self.my_life` (- (`self.my_life`) Damage))
  (if (<= (`self.my_life`) 0.0)
    (set `self.die?` true)))

(fn `atacando`
  (params (status :type Boolean))
  (if status
    (`|SpawnActorFromClass` "/Game/enemigos/esqueleto/proyectil_esqueleto_prqueBP.proyectil_esqueleto_prqueBP_C" (`SceneComponent.K2_GetComponentToWorld` (`self.Arrow1`)) "Undefined" "OverrideRootScale" null null)
    (else
      (set `self.ataco?` false))))

(fn `UserConstructionScript`)

(fn `velocidad`
  (params (velocidad :type "Float (double-precision)"))
  (set `CharacterMovementComponent.MaxWalkSpeed` velocidad (`self.CharacterMovement`)))